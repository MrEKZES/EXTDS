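; BP_Enemy is an enemy Blueprint with a health value that is destroyed when it takes enough damage.
; On BeginPlay it stores its spawn location as StarterPoint, which this graph does not use further.
; A Damage event subtracts from Health, prints the new value, and destroys the actor once Health drops below zero.
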(event `self.ReceiveBeginPlay`
  (set `self.StarterPoint` (`self.K2_GetActorLocation`)))

(event `Damage`
  (params (Damage :type "Float (double-precision)"))
  (bind _output_get (set `self.Health` (- (`self.Health`) Damage)))
  (`KismetSystemLibrary.PrintString` (`KismetStringLibrary.Conv_DoubleToString` _output_get))
  (if (< (`self.Health`) 0.0)
    (`self.K2_DestroyActor`)))

(fn `UserConstructionScript`)