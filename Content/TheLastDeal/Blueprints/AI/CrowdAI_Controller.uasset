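; AI controller for crowd characters that reacts when its perception component detects or loses the player character (BP_ThirdPersonCharacter).
; On detection it stores the actor as Target and sends a See.Player event to its StateTree.
; On loss it saves the target's current location as LastLocation and clears Target, without sending an event.
; Each perception update also prints a debug string with the target name and sensed state.
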(event `self.AIPerception.OnTargetPerceptionInfoUpdated`
  (params (UpdateInfo :type "ActorPerceptionUpdateInfo Structure (by ref)"))
  (bind (_targetid _target _stimulus) (break `ActorPerceptionUpdateInfo` UpdateInfo))
  (bind (_age _expirationage _strength _stimuluslocation _receiverlocation _tag _bsuccessfullysensed) (break `AIStimulus` _stimulus))
  (cast `/Game/ThirdPerson/Blueprints/BP_ThirdPersonCharacter` _target)
  (`KismetSystemLibrary.PrintString` (`KismetStringLibrary.Concat_StrStr` (`KismetSystemLibrary.GetDisplayName` _target) (`KismetStringLibrary.Conv_BoolToString` _bsuccessfullysensed)))
  (if _bsuccessfullysensed
    (set `self.Target` _target)
    (`StateTreeComponent.SendStateTreeEvent` (`self.StateTreeAI`) (make `StateTreeEvent` (struct :`TagName` "See.Player")))
    (else
      (set `self.LastLocation` (`self.K2_GetActorLocation` (`self.Target`)))
      (set `self.Target` null))))

(fn `UserConstructionScript`)