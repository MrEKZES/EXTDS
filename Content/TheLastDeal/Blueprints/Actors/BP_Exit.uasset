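; BP_Exit is an exit zone that loads Lvl_MainShelter once the player character has stayed inside its trigger for a set time.
; Entering resets the countdown from SecondsToRetention, shows a WBP_ExitTimer widget and starts a looping 0.1-second timer.
; Each tick pushes the remaining time to the widget and decrements it, opening the level at zero.
; Leaving the trigger removes the widget and clears the timer, cancelling the exit.
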(event `self.Trigger.OnComponentBeginOverlap`
  (params (OverlappedComponent :type "PrimitiveComponent Object Reference") (OtherActor :type "Actor Object Reference") (OtherComp :type "PrimitiveComponent Object Reference") (OtherBodyIndex :type Integer) (bFromSweep :type Boolean) (SweepResult :type "HitResult Structure (by ref)"))
  (cast `/Game/ThirdPerson/Blueprints/BP_ThirdPersonCharacter` OtherActor)
  (set `self.TempSeconds` (`self.SecondsToRetention`))
  (bind _returnvalue (`|CreateWidget` "/Game/TheLastDeal/Blueprints/UI/WBP_ExitTimer.WBP_ExitTimer_C"))
  (bind _output_get (set `self.TimerWidget` _returnvalue))
  (`UserWidget.AddToViewport` _output_get 0)
  (bind _returnvalue_2 (`KismetSystemLibrary.K2_SetTimerDelegate` (delegate `ReverseTimer`) 0.1 true))
  (set `self.Timer` _returnvalue_2))

(event `ReverseTimer`
  (set `/Game/TheLastDeal/Blueprints/UI/WBP_ExitTimer.Time` (`self.TempSeconds`) (`self.TimerWidget`))
  (set `self.TempSeconds` (- (`self.TempSeconds`) 0.1))
  (if (<= (`self.TempSeconds`) 0.0)
    (`GameplayStatics.OpenLevel` "Lvl_MainShelter")))

(event `self.Trigger.OnComponentEndOverlap`
  (params (OverlappedComponent :type "PrimitiveComponent Object Reference") (OtherActor :type "Actor Object Reference") (OtherComp :type "PrimitiveComponent Object Reference") (OtherBodyIndex :type Integer))
  (bind _timerwidget (`self.TimerWidget`))
  (cast `/Game/ThirdPerson/Blueprints/BP_ThirdPersonCharacter` OtherActor)
  (`/Engine/EditorBlueprintResources/StandardMacros.IsValid` _timerwidget
    (:`Is Valid`
      (`Widget.RemoveFromParent` _timerwidget)
      (`KismetSystemLibrary.K2_ClearAndInvalidateTimerHandle` (`self.Timer`)))))

(fn `UserConstructionScript`)